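; BP_Button_Base is a base button actor that animates its Button component back and forth and sets up its material.
; The construction script creates a dynamic instance of M_BaseButton on the Button and stores it in ButtonMaterial.
; From BeginPlay, two chained, eased MoveComponentTo calls shift the Button along relative Y and back, looping endlessly without using Tick.
; No press or interaction logic is present.
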(event EventBeginPlay
  (bind _button (Variables|Default|GetButton))
  (bind _relativelocation (Variables|/Script/Engine.SceneComponent|GetRelativeLocation _button))
  (Components|MoveComponentTo (Variables|Default|GetButton) (+ _relativelocation "0,10.000000,0.000000") "0, 0, 0" true true 2.0 false :!label _label)
  (Components|MoveComponentTo (Variables|Default|GetButton) (- _relativelocation "0,10.000000,0.000000") "0, 0, 0" true true 2.0 false)
  (goto _label))

(event EventTick
  (params (DeltaSeconds :type Float%20%28single-precision%29)))

(fn ConstructionScript
  (|InitializeButtonMaterial))