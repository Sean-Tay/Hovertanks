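; Scene-capture rig for a 3D button that renders a child actor into a texture-backed material.
; Construction colors a HollowCube, creates the capture's render target, and feeds it into a final dynamic material.
; The cube's Color doubles as that material's MaskColor, suggesting chroma-key masking of the background.
; BeginPlay adds the child actor to the show-only list, and Tick recaptures the scene every frame.
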(event EventTick
  (params (DeltaSeconds :type Float%20%28single-precision%29))
  (Rendering|SceneCapture|CaptureScene (Variables|Default|GetSceneCaptureComponent2D) :!class /Script/Engine.SceneCaptureComponent2D))

(event EventBeginPlay
  (Utilities|Array|Add (Variables|/Script/Engine.SceneCaptureComponent|GetShowOnlyActors (Variables|Default|GetSceneCaptureComponent2D)) (Variables|/Script/Engine.ChildActorComponent|GetChildActor (Variables|Default|GetActorToRender))))

(fn ConstructionScript
  (Utilities|FlowControl|Sequence
    (:then_0
      (bind _returnvalue (Rendering|Material|CreateDynamicMaterialInstance (Variables|Default|GetHollowCube) 0 "/Game/Utility/Objects/3D_Button/SceneCapture/M_Button_Scene_Capture.M_Button_Scene_Capture" :!class /Script/Engine.PrimitiveComponent))
      (bind _output_get (Variables|Default|SetHollowCubeDMI _returnvalue))
      (Rendering|Material|SetVectorParameterValue _output_get "Color" (Variables|Default|GetColor) :!class /Script/Engine.MaterialInstanceDynamic))
    (:then_1
      (bind _returnvalue_2 (Rendering|CreateRenderTarget2D 1024 1024))
      (Variables|Default|SetRenderTarget2D _returnvalue_2)
      (Variables|/Script/Engine.SceneCaptureComponent2D|SetTextureTarget (Variables|Default|GetSceneCaptureComponent2D) (Variables|Default|GetRenderTarget2D)))
    (:then_2
      (bind _returnvalue_3 (Rendering|Material|CreateDynamicMaterialInstance "/Game/Utility/Objects/3D_Button/SceneCapture/M_Button_Capture.M_Button_Capture" :!class /Script/Engine.KismetMaterialLibrary))
      (bind _output_get_2 (Variables|Default|SetFinalRenderTarget2DDMI _returnvalue_3))
      (Rendering|Material|SetTextureParameterValue _output_get_2 "RenderTarget2DInput" (Variables|Default|GetRenderTarget2D))
      (Rendering|Material|SetVectorParameterValue (Variables|Default|GetFinalRenderTarget2DDMI) "MaskColor" (Variables|Default|GetColor) :!class /Script/Engine.MaterialInstanceDynamic))))