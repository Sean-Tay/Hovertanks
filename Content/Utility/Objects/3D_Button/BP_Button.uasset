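; BP_Button is a 3D menu button that bobs back and forth and displays the option selected by UI type and index.
; UpdateButtonData picks a texture array, plays a change sound and sets the texture on a dynamic material.
; MenuSelect, gated by Activate/Deactivate, plays a sound and emissive pulse timeline, then a resettable DoOnce guards the action.
; Only Main Menu has actions: open the Desert level or quit, both with camera fade.
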(event EventBeginPlay
  (bind _button (Variables|Default|GetButton))
  (bind _relativelocation (Variables|/Script/Engine.SceneComponent|GetRelativeLocation _button))
  (Components|MoveComponentTo (Variables|Default|GetButton) (+ _relativelocation "0,10.000000,0.000000") "0, 0, 0" true true 2.0 false :!label _label)
  (Components|MoveComponentTo (Variables|Default|GetButton) (- _relativelocation "0,10.000000,0.000000") "0, 0, 0" true true 2.0 false)
  (goto _label))

(event EventTick
  (params (DeltaSeconds :type Float%20%28single-precision%29)))

(event Custom|Event%20Activate
  (Rendering|SetVisibility (Variables|Default|GetButton) true false)
  (Variables|Default|SetCanReceiveInput true))

(event Custom|Event%20Deactivate
  (Rendering|SetVisibility (Variables|Default|GetButton) false false)
  (Variables|Default|SetCanReceiveInput false))

(event Input|ActionEvents|InputActionMenuSelect
  (params (Key :type Key%20Structure :default "AnyKey"))
  (:Pressed
    (CallFunction|ExecuteButton)))

(event Custom|Execute%20Button
  (if (Variables|Default|GetCanReceiveInput)
    (Audio|PlaySound2D "/Game/Utility/Objects/3D_Button/SoundWaves/SW_ButtonSelect.SW_ButtonSelect")
    (bind _emissive_intensity (Timeline|PulseButton PlayFromStart)
      (:Update
        (Rendering|Material|SetScalarParameterValue (Variables|Default|GetButtonMaterial) "Emissive Multiplier" _emissive_intensity :!class /Script/Engine.MaterialInstanceDynamic))
      (:Execute
        (Utilities|FlowControl|DoOnce false
          (:Completed
            (switch Utilities|FlowControl|Switch|SwitchonEnum_UI_Type (Variables|Default|GetCurrentUI)
              (:NewEnumerator0
                (switch int (Variables|Default|GetCurrentIndex)
                  (:0
                    (Input|SetInputModeGameOnly (Game|GetPlayerController 0))
                    (Utilities|CameraFadeandDelay)
                    (Game|OpenLevel(byName) "Desert"))
                  (:1
                    (Utilities|CameraFadeandDelay)
                    (Game|QuitGame 0 "Quit")
                    (Development|ExecuteConsoleCommand "EXIT")))))))))))

(event Custom|AllowButtonExecution
  (Utilities|FlowControl|DoOnce false) ; enters at Reset
)

(fn ConstructionScript
  (|InitializeButtonMaterial)
  (CallFunction|UpdateButtonData (Variables|Default|GetCurrentUI) (Variables|Default|GetCurrentIndex)))

(fn UpdateButtonData
  (params (UI%20Type :type Enum_UI_Type%20Enum) (Index :type Integer))
  (Variables|Default|SetCurrentUI UI%20Type)
  (LocalVariables|Set_Index Index)
  (switch Utilities|FlowControl|Switch|SwitchonEnum_UI_Type (Variables|Default|GetCurrentUI)
    (:NewEnumerator1
      (return))
    (:NewEnumerator0
      (LocalVariables|Set_ChosenTextureArray (Variables|Default|GetMainMenuTextureArray)))
    (:NewEnumerator2
      (LocalVariables|Set_ChosenTextureArray (Variables|Default|GetInGameTextureArray))))
  ;[1 1 1] Prevents Continuous Sound
  (if (== (Variables|Default|GetCurrentIndex) (LocalVariables|Get_Index))
    _
    (else
      (Audio|PlaySound2D "/Game/Utility/Objects/3D_Button/SoundWaves/SW_ButtonChange.SW_ButtonChange")))
  (Variables|Default|SetCurrentIndex (Math|Integer|%(Integer) (LocalVariables|Get_Index) (Utilities|Array|Length (LocalVariables|Get_ChosenTextureArray))))
  (Utilities|SetTexture (Utilities|Array|Get(acopy) (LocalVariables|Get_ChosenTextureArray) (Variables|Default|GetCurrentIndex))
    (:OutputPin
      (return))))