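; Main menu pawn with a MouseRotationPoint and a Cursor component, whose event graph currently does nothing at runtime.
; Its tick and mouse axis events are empty.
; Disconnected logic would rotate MouseRotationPoint from axis input, then line trace forward along the Visibility channel to place Cursor at the hit or the trace end.
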(event EventBeginPlay)

(event EventActorBeginOverlap
  (params (OtherActor :type Actor%20Object%20Reference)))

(event EventTick
  (params (DeltaSeconds :type Float%20%28single-precision%29)))

(event Input|AxisEvents|InputAxisMouseHorizontal
  (params (AxisValue :type Float%20%28single-precision%29)))

(event Input|AxisEvents|InputAxisMouseVertical
  (params (AxisValue :type Float%20%28single-precision%29)))

(fn ConstructionScript)