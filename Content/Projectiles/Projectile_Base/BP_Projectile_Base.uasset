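; Base projectile Blueprint for a tank game that damages tanks on impact and expires after a short timer.
; Its collision sphere ignores itself, the firer and the owner while moving, and hits record location and normal.
; Tank hits apply damage and destroy it, projectile hits destroy only those tagged "Destructable", and other hits destroy it.
; A DoOnce-guarded Destroy stops movement and removes the sphere before destroying the actor.
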(event Custom|Destroy
  (Utilities|FlowControl|DoOnce false
    (:Completed
      (Components|Movement|StopMovementImmediately (Variables|Default|GetProjectileMovement))
      (Components|DestroyComponent (Variables|Default|GetSphere))
      (CallFunction|Destructor))))

(event EventBeginPlay
  (Utilities|Time|SetTimerbyEvent (delegate Custom|Destroy) 5.0)
  (|InitializeCollisionSphereToIgnoreCertainItems))

(event EventTick
  (params (DeltaSeconds :type Float%20%28single-precision%29)))

(fn ConstructionScript)

(fn Destructor
  (Actor|DestroyActor))

(event OnComponentHit(Sphere)
  (params (OtherActor :type Actor%20Object%20Reference) (OtherComp :type Primitive%20Component%20Object%20Reference) (NormalImpulse :type Vector :default "0, 0, 0") (Hit :type Hit%20Result%20Structure%20%28by%20ref%29))
  (bind (_bblockinghit _binitialoverlap _time _location _impactpoint _normal _impactnormal) (Collision|BreakHitResult Hit))
  (|CheckForSelfCollisions OtherActor)
  (Variables|Default|SetCollisionLocation _location)
  (Variables|Default|SetCollisionNormal _impactnormal)
  (|CastAndDamageTank OtherActor
    (:CastFailed
      (|CastAndDestroyProjectiles OtherActor
        (:CastFailed
          (Development|PrintString (Utilities|String|BuildString(Object) "" "Hit with: " OtherActor " !"))
          (CallFunction|Destroy))))))