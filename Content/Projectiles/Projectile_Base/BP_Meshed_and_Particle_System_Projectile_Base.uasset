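; Base projectile Blueprint that, going by its name, pairs a mesh with a particle system, extending a parent projectile class.
; Its Destructor override deactivates the particle system, destroys the Projectile component and spawns the explosion, then waits four seconds before calling the parent Destructor.
; The explosion emitter, if one is set, spawns at the collision location, nudged outward along the hit normal.
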(event EventBeginPlay)

(event EventActorBeginOverlap
  (params (OtherActor :type Actor%20Object%20Reference)))

(event EventTick
  (params (DeltaSeconds :type Float%20%28single-precision%29)))

(event EventDestructor
  (Components|Activation|Deactivate (Variables|Default|GetParticleSystem))
  (Components|DestroyComponent (Variables|Default|GetProjectile))
  (|spawnExplosion)
  (Utilities|FlowControl|Delay 4.0)
  (|CallParentFunction))

(fn ConstructionScript
  (|CallParentFunction))