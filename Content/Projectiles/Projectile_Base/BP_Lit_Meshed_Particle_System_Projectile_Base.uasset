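; Base Blueprint for lit projectiles with a mesh, particle trail and point light, extending a parent projectile class.
; Construction scales light intensity by a global brightness multiplier from a Material Parameter Collection.
; BeginPlay spawns an optional muzzle emitter ahead of the actor.
; Its Destructor event shuts down trail, mesh and light, spawns an optional explosion offset along the collision normal, then delays the parent destructor.
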(event EventBeginPlay
  (|spawnMuzzleFire)
  (|CallParentFunction))

(event EventActorBeginOverlap
  (params (OtherActor :type Actor%20Object%20Reference)))

(event EventTick
  (params (DeltaSeconds :type Float%20%28single-precision%29)))

(event EventDestructor
  (Components|Activation|Deactivate (Variables|Default|GetParticleSystemProjectileTrail))
  (Components|DestroyComponent (Variables|Default|GetProjectile))
  (Rendering|SetVisibility (Variables|Default|GetPointLight) false false)
  (|spawnExplosion)
  (Utilities|FlowControl|Delay 4.0)
  (|CallParentFunction))

(fn ConstructionScript
  (bind _pointlight (Variables|Default|GetPointLight))
  (|CallParentFunction)
  (bind _returnvalue (Rendering|Material|GetScalarParameterValue "/Game/Utility/MPC_GlobalParameters.MPC_GlobalParameters" "GlobalLightBrightnessMultiplier" :!class /Script/Engine.KismetMaterialLibrary))
  (Rendering|Components|Light|SetIntensity _pointlight (* (Variables|/Script/Engine.LightComponentBase|GetIntensity _pointlight) _returnvalue)))