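; Base tank weapon holder that manages the current weapon's state, mesh, ammunition and firing, with empty fire and animation hooks.
; ChangeWeapon stores a WeaponState and sets its mesh; Reload adds matching-type ammo up to maximum capacity.
; Fire accepts positive or -1 capacity, decrements it and uses DoOnce plus Delay for recharge, otherwise printing a throttled out-of-ammo message.
; A disabled flag, toggled by Enable and Disable, gates these events.
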(event EventBeginPlay)

(event EventTick
  (params (DeltaSeconds :type Float%20%28single-precision%29)))

(fn ConstructionScript)

(fn FireWeapon)

(fn ReloadWeapon
  (params (Ammo :type BP%20Weapon%20Refill%20Base%20Object%20Reference)))

(fn UnloadWeapon
  (if (== (Variables|Default|GetStaticMesh) 0)
    _))

(fn LoadWeapon
  (params (Static%20Mesh :type Static%20Mesh%20Object%20Reference))
  (Components|StaticMesh|SetStaticMesh (Variables|Default|GetStaticMesh) Static%20Mesh))

(event Custom|ChangeWeapon
  (params (Weapon%20State :type Struct%20Weapon%20State%20Structure))
  (Utilities|DisallowExecutionifDisabled)
  (bind _output_get (Variables|Default|SetWeaponState Weapon%20State))
  (CallFunction|UnloadWeapon)
  (CallFunction|LoadWeapon (.WeaponMesh (Utilities|Struct|BreakStruct_Weapon_State _output_get))))

(event Custom|Reload
  (params (Ammo :type BP%20Weapon%20Refill%20Base%20Object%20Reference))
  (Utilities|DisallowExecutionifDisabled)
  (|IfAmmoTypeAndWeaponTypeAreTheSame Ammo
    (:true
      (|AddAmmoIntoWeaponState Ammo))))

(event Custom|Fire
  (Utilities|DisallowExecutionifDisabled)
  (|CheckforEnoughAmmunition
    (:true
      (|FireTheWeapon))
    (:false
      (|PrintOutofAmmunitionMessage))))

(event Custom|Enable
  (Utilities|IsDisabledActive
    (:true
      (Variables|Default|SetisDisabled false))))

(event Custom|Disable
  (Utilities|IsDisabledActive
    (:false
      (Variables|Default|SetisDisabled true))))

(event Custom|FiringAnimation
  (Utilities|DisallowExecutionifDisabled))