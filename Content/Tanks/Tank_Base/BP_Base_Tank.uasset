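; Base hover tank Blueprint that handles physics movement, turret aiming, health and hover setup.
; On BeginPlay it loads per-type stats from the game instance and uses them to configure its hover modules, with softer force front and back.
; Tick derives grounded state from module hits and aligns four corner modules to the turret.
; Input drives thrust along turret forward, body torque and clamped aiming, with different movement force and torque when airborne.
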(event EventTick
  (params (DeltaSeconds :type Float%20%28single-precision%29))
  (|UpdateTankPositionalData))

(event EventBeginPlay
  (|InitializeTankStats)
  (|InitializeHovering))

(fn ConstructionScript
  (|InitializeHoverModuleArray))

(fn IsTurretRotationAllowable
  (return (Math|Float|NearlyEqual(Float) (Math|Vector|DotProduct (Math|Vector|GetForwardVector (Variables|Default|GetBody)) (Math|Vector|GetForwardVector (Variables|Default|GetTurret))) 1.0 0.5)))

(fn TurnBodyLaterally
  (params (Axis%20Value :type Float%20%28single-precision%29))
  (bind _body (Variables|Default|GetBody))
  (bind _returnvalue (Physics|GetPhysicsLinearVelocity _body "None"))
  (if (Variables|Default|GetisNotInAir)
    (Class|PrimitiveComponent|AddTorque _body (Math|Vector|MakeVector 0.0 0.0 (* Axis%20Value (.baserotationspeed (Variables|Default|GetTankStats)))) "None" true)
    (else
      (Class|PrimitiveComponent|AddTorque (Variables|Default|GetBody) (Math|Vector|MakeVector 0.0 0.0 (* Axis%20Value 5.0)) "None" true)))
  (return))

(fn GetHoverTanksGameInstance
  (bind _ashovertanks_game_instance (Utilities|Casting|CastToHovertanks_Game_Instance (Game|GetGameInstance))
    (:then
      (return _ashovertanks_game_instance true))
    (:CastFailed
      (return 0 false))))

(fn GetWeaponHolderOutOfChildActor
  (params (Child%20Actor%20Reference :type Child%20Actor%20Component%20Object%20Reference))
  (bind _asbp_weapon_holder (Utilities|Casting|CastToBP_Weapon_Holder (Variables|/Script/Engine.ChildActorComponent|GetChildActor Child%20Actor%20Reference))
    (:then
      _)
    (:CastFailed
      _))
  (return _asbp_weapon_holder))

(event Custom|Load%20Tank%20State
  (bind (_game_instance _success) (CallFunction|GetHoverTanksGameInstance))
  (if _success
    (bind _tankstats (Default|ReturnTemplateTankStatsforSpecifiedTankType _game_instance (Variables|Default|GetTankType)))
    (Variables|Default|SetTankStats _tankstats)
    (else
      (Development|PrintString "Unable to load Tank Stats"))))

(event Input|AxisEvents|InputAxisMouseHorizontal
  (params (AxisValue :type Float%20%28single-precision%29))
  (bind _turret (Variables|Default|GetTurret))
  (bind _tankstats (Variables|Default|GetTankStats))
  (bind _returnvalue (* AxisValue (.baseturretspeed _tankstats)))
  (Transformation|AddLocalRotation _turret (Math|Rotator|MakeRotator 0.0 0.0 _returnvalue) false false)
  ;[1 1 1] Restrict Turret Rotation if Rotation Exceeds Boundaries
  (if (not (Math|Float|InRange(Float) (.yaw (Variables|/Script/Engine.SceneComponent|GetRelativeRotation _turret)) -45.0 45.0))
    (Transformation|AddLocalRotation (Variables|Default|GetTurret) (Math|Rotator|MakeRotator 0.0 0.0 (* _returnvalue -1.0)) false false)))

(event Custom|RepairTank
  (params (Amount :type Float%20%28single-precision%29))
  (Variables|Default|SetHealthPoints (Math|Float|Min(Float) (+ Amount (Variables|Default|GetHealthPoints)) (.maxhealthpoints (Variables|Default|GetTankStats)))))

(event Input|AxisEvents|InputAxisMouseVertical
  (params (AxisValue :type Float%20%28single-precision%29))
  (bind _y_axis_rotation_point (Variables|Default|GetY_Axis_Rotation_Point))
  (bind _tankstats (Variables|Default|GetTankStats))
  (bind _returnvalue (* AxisValue (.baseturretspeed _tankstats)))
  (Transformation|AddLocalRotation _y_axis_rotation_point (Math|Rotator|MakeRotator 0.0 _returnvalue 0.0) false false)
  ;[1 1 1] Restrict Y_Axis_Rotation_Point if Rotation Exceeds Boundaries
  (if (not (Math|Float|InRange(Float) (.pitch (Variables|/Script/Engine.SceneComponent|GetRelativeRotation _y_axis_rotation_point)) -5.0 25.0))
    (Transformation|AddLocalRotation (Variables|Default|GetY_Axis_Rotation_Point) (Math|Rotator|MakeRotator 0.0 (* _returnvalue -1.0) 0.0) false false)))

(event Custom|DamageTank
  (params (Amount :type Float%20%28single-precision%29))
  (|IsHealthPointsBelow0AfterCalculations (- (Variables|Default|GetHealthPoints) Amount)
    (:true)
    (:false
      (Variables|Default|SetHealthPoints (- (Variables|Default|GetHealthPoints) Amount)))))

(event Input|AxisEvents|InputAxisForward
  (params (AxisValue :type Float%20%28single-precision%29))
  (bind _tankstats (Variables|Default|GetTankStats))
  (bind _body (Variables|Default|GetBody))
  (bind _turret (Variables|Default|GetTurret))
  (bind _returnvalue (Math|Vector|GetForwardVector _turret))
  (bind _returnvalue_2 (* (.basemovespeed _tankstats) AxisValue))
  (bind _returnvalue_3 (* _returnvalue 5e+05))
  (bind _returnvalue_4 (* _returnvalue_3 _returnvalue_2))
  (if (Variables|Default|GetisNotInAir)
    (Class|PrimitiveComponent|AddForceatLocation _body _returnvalue_4 (+ (Transformation|GetWorldLocation _body) (Math|Vector|MakeVector -1.0 0.0 -1.0)) "None")
    (else
      (Physics|AddForce _body (* _returnvalue_4 0.3) "None" false))))

(event Custom|TurnByTurret
  (params (Axis%20Value :type Float%20%28single-precision%29))
  (CallFunction|TurnBodyLaterally Axis%20Value))

(event Input|AxisEvents|InputAxisRight
  (params (AxisValue :type Float%20%28single-precision%29))
  (CallFunction|TurnBodyLaterally AxisValue))