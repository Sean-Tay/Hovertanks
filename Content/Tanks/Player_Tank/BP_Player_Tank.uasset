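; Player hover tank Blueprint that manages a paired primary weapon loadout and a single secondary weapon, each held in a child-actor weapon holder.
; On BeginPlay it loads weapon state from the GameInstance, which it can also save back, and equips the holders.
; Input toggles fire and change flags that Tick polls, copying holder state back into the arrays, cycling weapons with a one-second cooldown, and firing.
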(event EventBeginPlay
  (|CallParentFunction)
  (|InitializeWeaponry))

(event EventActorBeginOverlap
  (params (OtherActor :type Actor%20Object%20Reference)))

(event EventTick
  (params (DeltaSeconds :type Float%20%28single-precision%29))
  (|CallParentFunction 0.0)
  (|UpdateWeapons))

(fn ConstructionScript
  (|CallParentFunction))

(event Custom|Save%20Weapon%20State
  (bind (_game_instance _success) (CallFunction|GetHoverTanksGameInstance))
  (if _success
    (Variables|/Game/Hovertanks_Game_Instance.Hovertanks_Game_Instance_C|SetPlayerWeaponState _game_instance (Variables|Default|GetTankWeaponState))
    (else
      (Development|PrintString "Unable to save Weapon State"))))

(event Custom|Add%20Weapon
  (params (New%20Weapon :type Struct%20Weapon%20State%20Structure))
  (switch Utilities|FlowControl|Switch|SwitchonEnum_Weapon_Priority (.WeaponPriority (Utilities|Struct|BreakStruct_Weapon_State New%20Weapon))
    (:NewEnumerator0
      (Utilities|Array|Add (.primaryweaponarray (Variables|Default|GetTankWeaponState)) (Utilities|WeaponStateStructDuplicator New%20Weapon))
      (Utilities|Array|Add (.primaryweaponarray (Variables|Default|GetTankWeaponState)) (Utilities|WeaponStateStructDuplicator New%20Weapon)))
    (:NewEnumerator1
      (Utilities|Array|AddUnique (.secondaryweaponarray (Variables|Default|GetTankWeaponState)) New%20Weapon))))

(event Custom|Load%20Weapon%20State
  (bind (_game_instance _success) (CallFunction|GetHoverTanksGameInstance))
  (if _success
    (Variables|Default|SetTankWeaponState (Variables|/Game/Hovertanks_Game_Instance.Hovertanks_Game_Instance_C|GetPlayerWeaponState _game_instance))
    (else
      (Development|PrintString "Unable to load Weapon State"))))

(event Input|ActionEvents|InputActionChangePrimaryWeapon
  (params (Key :type Key%20Structure :default "AnyKey"))
  (:Pressed
    (Variables|Default|SetisChangingPrimaryWeapon (not (Variables|Default|GetisChangingPrimaryWeapon)) :!label _label))
  (:Released
    (goto _label)))

(event Input|ActionEvents|InputActionChangeSecondaryWeapon
  (params (Key :type Key%20Structure :default "AnyKey"))
  (:Pressed
    (Variables|Default|SetisChangingSecondaryWeapon (not (Variables|Default|GetisChangingSecondaryWeapon)) :!label _label))
  (:Released
    (goto _label)))

(event Input|ActionEvents|InputActionFireSecondaryWeapon
  (params (Key :type Key%20Structure :default "AnyKey"))
  (:Pressed
    (Variables|Default|SetisFiringSecondaryWeapon (not (Variables|Default|GetisFiringSecondaryWeapon)) :!label _label))
  (:Released
    (goto _label)))

(event Input|ActionEvents|InputActionFirePrimaryWeapon
  (params (Key :type Key%20Structure :default "AnyKey"))
  (:Pressed
    (Variables|Default|SetisFiringPrimaryWeapon (not (Variables|Default|GetisFiringPrimaryWeapon)) :!label _label))
  (:Released
    (goto _label)))