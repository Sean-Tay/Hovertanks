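; BP_Weapon_Inventory_Object holds a player tank's weapons as an array of weapon state objects and tracks the active one by index.
; Adding a weapon converts a weapon state struct into an object owned by the inventory before storing it.
; Switching cycles the index with wraparound and returns the new state, while removal works by index or reference and clamps the index to the last entry.
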(fn Initialize
  (bind _output_get (Variables|Default|SetWeaponStateArray (Utilities|Array|MakeArray 0)))
  (Utilities|Array|Clear _output_get)
  (Variables|Default|SetCurrentIndex 0)
  (return))

(fn GetCurrentWeaponState
  (return (Utilities|Array|Get(acopy) (Variables|Default|GetWeaponStateArray) (Variables|Default|GetCurrentIndex))))

(fn AddWeaponState
  (params (Weapon%20State%20Struct :type Struct%20Weapon%20State%20Structure))
  (bind _weapon_state_object (Utilities|WeaponStateStructtoObject self Weapon%20State%20Struct))
  (Utilities|Array|Add (Variables|Default|GetWeaponStateArray) _weapon_state_object)
  (return))

(fn RemoveWeaponState
  (params (Index :type Integer) (Weapon%20State :type BP%20Weapon%20State%20Object%20Object%20Reference) (Use%20Index :type Boolean))
  (if Use%20Index
    (Utilities|Array|RemoveIndex (Variables|Default|GetWeaponStateArray) Index)
    (else
      (Utilities|Array|RemoveItem (Variables|Default|GetWeaponStateArray) Weapon%20State)))
  (Variables|Default|SetCurrentIndex (Math|Integer|Min(Integer) (Variables|Default|GetCurrentIndex) (- (Utilities|Array|Length (Variables|Default|GetWeaponStateArray)) 1)))
  (return))

(fn SwitchWeapon
  (bind _output_get (Variables|Default|SetCurrentIndex (Math|Integer|%(Integer) (+ (Variables|Default|GetCurrentIndex) 1) (Utilities|Array|Length (Variables|Default|GetWeaponStateArray)))))
  (return (Utilities|Array|Get(acopy) (Variables|Default|GetWeaponStateArray) _output_get)))