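; BP_Weapon_State_Object is a data object that holds one weapon's state in a WeaponState struct.
; Getter functions expose its mesh, priority, type, class, capacity, recharge time, and UI data such as icon, reticle and color.
; Current capacity is the only field with a setter, which writes it back into the struct.
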(fn GetWeaponMesh
  (return (.WeaponMesh (Utilities|Struct|BreakStruct_Weapon_State (Variables|Default|GetWeaponStateStruct)))))

(fn GetWeaponPriority
  (return (.WeaponPriority (Utilities|Struct|BreakStruct_Weapon_State (Variables|Default|GetWeaponStateStruct)))))

(fn GetWeaponType
  (return (.WeaponType (Utilities|Struct|BreakStruct_Weapon_State (Variables|Default|GetWeaponStateStruct)))))

(fn GetWeaponClass
  (return (.WeaponClass (Utilities|Struct|BreakStruct_Weapon_State (Variables|Default|GetWeaponStateStruct)))))

(fn GetCurrentCapacity
  (return (.CurrentCapacity (Utilities|Struct|BreakStruct_Weapon_State (Variables|Default|GetWeaponStateStruct)))))

(fn GetMaximumCapacity
  (return (.MaximumCapacity (Utilities|Struct|BreakStruct_Weapon_State (Variables|Default|GetWeaponStateStruct)))))

(fn GetRechargeTime
  (return (.RechargeTime (Utilities|Struct|BreakStruct_Weapon_State (Variables|Default|GetWeaponStateStruct)))))

(fn SetCurrentCapacity
  (params (Capacity :type Integer))
  (Utilities|Struct|SetmembersinStruct_Weapon_State (Variables|Default|GetWeaponStateStruct) Capacity)
  (return))

(fn GetWeaponIcon
  (return (.weaponicon (Variables|Default|GetWeaponStateStruct))))

(fn GetWeaponReticle
  (return (.weaponreticle (Variables|Default|GetWeaponStateStruct))))

(fn GetWeaponColor
  (return (.weaponcolor (Variables|Default|GetWeaponStateStruct))))