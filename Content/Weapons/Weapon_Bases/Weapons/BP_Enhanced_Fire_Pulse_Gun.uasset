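; Enhanced pulse gun weapon Blueprint that extends a parent weapon's Fire to launch enhanced rapid pulse projectiles.
; Each shot passes a DoOnce gate and ammo check, then spawns the projectile with its effects, sound, firer and direction, and plays a camera shake.
; A recoil timeline, rate-scaled by the weapon state's recharge time, kicks the mesh backward and reopens the gate on finish, so it doubles as the cooldown.
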(event EventTick
  (params (DeltaSeconds :type Float%20%28single-precision%29))
  (|CallParentFunction 0.0))

(event EventEnable
  (|CallParentFunction))

(event EventDisable
  (|CallParentFunction))

(event EventFire
  (|CallParentFunction)
  (Utilities|FlowControl|DoOnce false :!label _label
    (:Completed
      (bind _canfire (CallFunction|CheckandDecrementAmmoCount))
      (if _canfire
        (bind _returnvalue (CallFunction|CalculateForwardDirectionVector))
        (Game|SpawnActorfromClass "/Game/Projectiles/Projectile_Classes/BP_Enhanced_Rapid_Pulse_Gun_Projectile.BP_Enhanced_Rapid_Pulse_Gun_Projectile_C" (Transformation|GetWorldTransform (Variables|Default|GetLocalForwardPoint)) "Undefined" 0 "/Game/Projectiles/Projectile_Skins/ParticleSystems/PulseGuns/PS_EnhancedRapidFirePulseGunMuzzleFire.PS_EnhancedRapidFirePulseGunMuzzleFire" "/Game/Projectiles/Projectile_Skins/ParticleSystems/PulseGuns/PS_EnhancedRapidFirePulseGunExplosion.PS_EnhancedRapidFirePulseGunExplosion" (Variables|Default|GetFirer) _returnvalue "/Game/Projectiles/Audio/PulseGuns/SC_PulseGun.SC_PulseGun")
        (Camera|PlayWorldCameraShake "/Game/Utility/CustomCameraShake.CustomCameraShake_C" (Transformation|GetActorLocation) 0.0 0.0)
        (bind _rechargetime (Default|GetRechargeTime (Variables|Default|GetWeapon%20State%20Object)))
        (Components|Timeline|SetPlayRate (Variables|Default|GetFiringAnimation) (/ 1.0 _rechargetime))
        (bind _recoilcurve (Timeline|FiringAnimation PlayFromStart)
          (:Update
            (bind _returnvalue_2 (CallFunction|CalculateForwardDirectionVector))
            (Transformation|SetRelativeLocation (Variables|Default|GetStaticMesh) (* (* _returnvalue_2 -75.0) _recoilcurve) false false))
          (:Finished
            (goto _label Reset)))
        (else
          (goto _label Reset))))))

(fn ConstructionScript
  (|CallParentFunction))