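; Base weapon Blueprint providing enable/disable state, aiming and ammunition logic, with Fire and FiringAnimation events that contain only a disabled-state check.
; GetAimLocation line-traces on Visibility from the root through LocalForwardPoint, returning the impact point or trace end.
; Ammo macros read and decrement capacity on WeaponStateObject, treating -1 as unlimited.
; An empty weapon prints an out-of-ammunition message, throttled by DoOnce and the recharge time.
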(event Custom|Fire
  (Utilities|DisallowExecutionifDisabled))

(event Custom|Enable
  (Variables|Default|SetisDisabled false))

(event Custom|Disable
  (Variables|Default|SetisDisabled true))

(event Custom|FiringAnimation
  (Utilities|DisallowExecutionifDisabled))

(event EventBeginPlay)

(event EventTick
  (params (DeltaSeconds :type Float%20%28single-precision%29)))

(fn ConstructionScript)

(fn GetAimLocation
  (bind _defaultsceneroot (Variables|Default|GetDefaultSceneRoot))
  (bind _returnvalue (Transformation|GetWorldLocation _defaultsceneroot))
  (bind _output_get (LocalVariables|SetAimVector (- _returnvalue (Transformation|GetWorldLocation (Variables|Default|GetLocalForwardPoint)))))
  (if (> (Math|Vector|VectorLength _output_get) 0.0)
    (LocalVariables|SetAimVector (* (LocalVariables|GetAimVector) -1)))
  (bind _outhit (Collision|LineTraceByChannel _returnvalue (+ _returnvalue (* (LocalVariables|GetAimVector) 65535)) "TraceTypeQuery1" false 0 "None"))
  (if (.bBlockingHit (Collision|BreakHitResult _outhit))
    (return (.ImpactPoint (Collision|BreakHitResult _outhit)))
    (else
      (return (.TraceEnd (Collision|BreakHitResult _outhit))))))