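; BP_Weapon_Holder is a weapon mount that swaps guns through a weapon state object supplying mesh, class, type, ammo and recharge time.
; Fire checks ammo (-1 means unlimited), then, for Discrete weapons only, spends a round, shakes the camera, plays timeline recoil and spawns a pulse-gun projectile by class.
; Enable/Disable events set a flag gating actions, and a line trace provides the aim point.
; Reloading is an empty stub.
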(event EventBeginPlay)

(event EventTick
  (params (DeltaSeconds :type Float%20%28single-precision%29)))

(fn ConstructionScript)

(fn ProduceProjectile
  (bind _forward_vector (Utilities|GetForwardDirectionVector))
  (bind _self self)
  (bind _firer (Variables|Default|GetFirer))
  (bind _firingpoint (Variables|Default|GetFiringPoint))
  (bind _returnvalue (Transformation|GetWorldTransform _firingpoint))
  (bind _weaponclass (Default|GetWeaponClass (Variables|Default|GetWeapon%20State%20Object)))
  (switch Utilities|FlowControl|Switch|SwitchonEnum_Weapon_Class _weaponclass
    (:NewEnumerator4
      (Game|SpawnActorfromClass "/Game/Projectiles/Projectile_Classes/BP_Rapid_Pulse_Gun_Projectile.BP_Rapid_Pulse_Gun_Projectile_C" _returnvalue "Undefined" _self "/Game/Projectiles/Projectile_Skins/ParticleSystems/PulseGuns/PS_RapidFirePulseGunMuzzleFire.PS_RapidFirePulseGunMuzzleFire" "/Game/Projectiles/Projectile_Skins/ParticleSystems/PulseGuns/PS_RapidFirePulseGunExplosion.PS_RapidFirePulseGunExplosion" _firer _forward_vector "/Game/Projectiles/Audio/PulseGuns/SC_PulseGun.SC_PulseGun"))
    (:NewEnumerator5
      (Game|SpawnActorfromClass "/Game/Projectiles/Projectile_Classes/BP_Enhanced_Rapid_Pulse_Gun_Projectile.BP_Enhanced_Rapid_Pulse_Gun_Projectile_C" _returnvalue "Undefined" _self "/Game/Projectiles/Projectile_Skins/ParticleSystems/PulseGuns/PS_EnhancedRapidFirePulseGunMuzzleFire.PS_EnhancedRapidFirePulseGunMuzzleFire" "/Game/Projectiles/Projectile_Skins/ParticleSystems/PulseGuns/PS_EnhancedRapidFirePulseGunExplosion.PS_EnhancedRapidFirePulseGunExplosion" _firer _forward_vector "/Game/Projectiles/Audio/PulseGuns/SC_PulseGun.SC_PulseGun"))))

(fn ReloadWeapon
  (params (Ammo :type BP%20Weapon%20Refill%20Base%20Object%20Reference)))

(fn UnloadWeapon
  (if (== (Variables|Default|GetStaticMesh) 0)
    _))

(fn LoadWeapon
  (params (Static%20Mesh :type Static%20Mesh%20Object%20Reference))
  (Components|StaticMesh|SetStaticMesh (Variables|Default|GetStaticMesh) Static%20Mesh))

(fn GetAimLocation
  (bind _defaultsceneroot (Variables|Default|GetDefaultSceneRoot))
  (bind _returnvalue (Transformation|GetWorldLocation _defaultsceneroot))
  (bind _output_get (LocalVariables|SetAimVector (- _returnvalue (Transformation|GetWorldLocation (Variables|Default|GetFiringPoint)))))
  (if (> (Math|Vector|VectorLength _output_get) 0.0)
    (LocalVariables|SetAimVector (* (LocalVariables|GetAimVector) -1)))
  (bind _outhit (Collision|LineTraceByChannel _returnvalue (+ _returnvalue (* (LocalVariables|GetAimVector) 1024)) "TraceTypeQuery1" false 0 "None"))
  (if (.bBlockingHit (Collision|BreakHitResult _outhit))
    (return (.ImpactPoint (Collision|BreakHitResult _outhit)))
    (else
      (return (.TraceEnd (Collision|BreakHitResult _outhit))))))

(event Custom|ChangeWeapon
  (params (Weapon%20State :type BP%20Weapon%20State%20Object%20Object%20Reference))
  (Utilities|DisallowExecutionifDisabled)
  (if (not (== Weapon%20State 0))
    (bind _output_get (Variables|Default|SetWeapon%20State%20Object Weapon%20State))
    (bind _weaponmesh (Default|GetWeaponMesh _output_get))
    (CallFunction|UnloadWeapon)
    (CallFunction|LoadWeapon _weaponmesh)))

(event Custom|Fire
  (Utilities|DisallowExecutionifDisabled)
  (|CheckforEnoughAmmunition
    (:true
      (|FireTheWeapon))
    (:false
      (|PrintOutofAmmunitionMessage))))

(event Custom|Enable
  (Utilities|IsDisabledActive
    (:true
      (Variables|Default|SetisDisabled false))))

(event Custom|Disable
  (Utilities|IsDisabledActive
    (:false
      (Variables|Default|SetisDisabled true))))

(event Custom|FiringAnimation
  (bind _weapon_state_object (Variables|Default|GetWeapon%20State%20Object))
  (Utilities|DisallowExecutionifDisabled)
  (bind _weapontype (Default|GetWeaponType _weapon_state_object))
  (switch Utilities|FlowControl|Switch|SwitchonEnum_Weapon_Type _weapontype
    (:NewEnumerator0
      (bind _rechargetime (Default|GetRechargeTime _weapon_state_object))
      (Components|Timeline|SetPlayRate (Variables|Default|GetRecoilTimeline) (/ 1.0 _rechargetime))
      (bind _recoilfloattrack (Timeline|RecoilTimeline PlayFromStart)
        (:Update
          (Transformation|SetRelativeLocation (Variables|Default|GetStaticMesh) (* (* (Utilities|GetForwardDirectionVector) -75.0) _recoilfloattrack) false false))
        (:Finished)))))